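; Player controller for a modular builder that spawns a module and lets the player position it in the world with the mouse.
; M spawns a VBS_ModuleBase with a preset mesh and marks it as being placed; R rotates it, with Shift reversing direction.
; Tick deprojects the cursor and moves the module along that ray at an adjustable, clamped distance, applying yaw in 90-degree phases.
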(event `Key|R`
  (params (Key :type "Key Structure"))
  (bind _moduilebeingplaced (`self.ModuileBeingPlaced`))
  (:`Pressed`
    (bind _result (`self.IsModuleBeingPlaced`))
    (if _result
      (if (or (`self.IsInputKeyDown` "LeftShift") (`self.IsInputKeyDown` "RightShift"))
        (`/Game/Builder/VBS_ModuleBase.RotateModule` _moduilebeingplaced false)
        (else
          (`/Game/Builder/VBS_ModuleBase.RotateModule` _moduilebeingplaced true))))))

(event `Key|M`
  (params (Key :type "Key Structure"))
  (:`Pressed`
    (`self.SpawnModuleForPlacing` "/Game/Builder/VBS_Mesh_ModuleA.VBS_Mesh_ModuleA")))

(event `InputAction|VBS_ModulePlacementDistanceINC`
  (params (Key :type "Key Structure"))
  (:`Pressed`
    (bind _result (`self.IsModuleBeingPlaced`))
    (if _result
      (set `self.ModulePlacementDistanceFromPlayer` (`KismetMathLibrary.FMin` (+ 10.0 (`self.ModulePlacementDistanceFromPlayer`)) 5000.0)))))

(event `InputAction|VBS_ModulePlacementDistanceDEC`
  (params (Key :type "Key Structure"))
  (:`Pressed`
    (bind _result (`self.IsModuleBeingPlaced`))
    (if _result
      (set `self.ModulePlacementDistanceFromPlayer` (`KismetMathLibrary.FMax` (- (`self.ModulePlacementDistanceFromPlayer`) 10.0) 100.0)))))

(event `self.ReceiveTick`
  (params (DeltaSeconds :type "Float (single-precision)"))
  (bind (_worldlocation _worlddirection _returnvalue) (`self.DeprojectMousePositionToWorld`))
  (bind _moduilebeingplaced (`self.ModuileBeingPlaced`))
  ;[1 1 1] If ModuleBeingPlaced is valid, adjust position and rotation as needed...
  (`/Engine/EditorBlueprintResources/StandardMacros.IsValid` _moduilebeingplaced
    (:`Is Valid`
      (if _returnvalue
        (`self.K2_SetActorTransform` _moduilebeingplaced (`KismetMathLibrary.MakeTransform` (+ _worldlocation (* _worlddirection (`self.ModulePlacementDistanceFromPlayer`))) (`KismetMathLibrary.MakeRotator` 0.0 0.0 (* (`KismetMathLibrary.Conv_ByteToDouble` (`/Game/Builder/VBS_ModuleBase.CurrentRotationPhase` (`self.ModuileBeingPlaced`))) 90.0))) false false)))))

(fn `IsModuleBeingPlaced`
  (returns (Result :type Boolean))
  (bind _moduilebeingplaced (`self.ModuileBeingPlaced`))
  (`/Engine/EditorBlueprintResources/StandardMacros.IsValid` _moduilebeingplaced
    (:`Is Valid`
      (if (`/Game/Builder/VBS_ModuleBase.IsBeingPlaced` _moduilebeingplaced)
        (return true)
        (else
          _)))
    (:`Is Not Valid`
      _))
  (return false))

(fn `SpawnModuleForPlacing`
  (params (`Module Type` :type "StaticMesh Object Reference"))
  (bind _returnvalue (`|SpawnActorFromClass` "/Game/Builder/VBS_ModuleBase.VBS_ModuleBase_C" (`KismetMathLibrary.MakeTransform` (0.0 0.0 0.0)) "AlwaysSpawn" "OverrideRootScale" null null))
  (set `/Game/Builder/VBS_ModuleBase.ModuleStaticMesh` `Module Type` _returnvalue)
  (`/Game/Builder/VBS_ModuleBase.UpdateCurrentMesh` _returnvalue)
  (`self.StartPlacingModule` _returnvalue))

(fn `StartPlacingModule`
  (params (ModuleToPlace :type "/Game/Builder/VBS_ModuleBase Object Reference"))
  (set `/Game/Builder/VBS_ModuleBase.IsBeingPlaced` true ModuleToPlace)
  (set `self.ModuileBeingPlaced` ModuleToPlace))

(fn `StopPlacingCurrentModule`
  (bind _moduilebeingplaced (`self.ModuileBeingPlaced`))
  (`/Engine/EditorBlueprintResources/StandardMacros.IsValid` _moduilebeingplaced
    (:`Is Valid`
      (set `/Game/Builder/VBS_ModuleBase.IsBeingPlaced` false _moduilebeingplaced)
      (set `self.ModuileBeingPlaced` null))))

(fn `UserConstructionScript`)