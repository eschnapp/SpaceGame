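; Player controller for the vessel editor that spawns a module and lets the player position it with the mouse.
; M spawns Module_A as the current module if none is valid, and Tick moves it along the deprojected cursor ray at an adjustable distance unless it is snapping.
; Add and Subtract change that distance with a lower limit, while R and Shift+R step the yaw in quarter turns in opposite directions.
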(event `self.ReceiveTick`
  (params (DeltaSeconds :type "Float (single-precision)"))
  (bind (_worldlocation _worlddirection) (`self.DeprojectMousePositionToWorld`))
  (bind _current_module (`self.Current Module`))
  (`/Engine/EditorBlueprintResources/StandardMacros.IsValid` _current_module
    (:`Is Valid`
      (if (not (`/Game/VesselEditor/ModuleBP.IsSnapping` _current_module))
        (`self.K2_SetActorTransform` _current_module (`KismetMathLibrary.MakeTransform` (+ _worldlocation (* _worlddirection (`self.Module Distance`))) (`KismetMathLibrary.MakeRotator` 0.0 0.0 (* (`self.ModuleRotationPhase`) 90.0))) false false)))))

(event `Key|M`
  (params (Key :type "Key Structure"))
  (:`Pressed`
    (`self.SpawnModule` "/Game/VesselEditor/Module_A.Module_A_C")))

(event `Key|Add`
  (params (Key :type "Key Structure"))
  (:`Pressed`
    (set `self.Module Distance` (+ (`self.Module Distance`) 10.0))))

(event `Key|Subtract`
  (params (Key :type "Key Structure"))
  (bind _returnvalue (- (`self.Module Distance`) 10.0))
  (:`Pressed`
    (set `self.Module Distance` (select `bool` (<= _returnvalue 100.0) :`false` _returnvalue :`true` 100.0))))

(event `Key|R`
  (params (Key :type "Key Structure"))
  (bind _modulerotationphase (`self.ModuleRotationPhase`))
  (:`Pressed`
    (if (or (`self.IsInputKeyDown` "LeftShift") (`self.IsInputKeyDown` "RightShift"))
      (set `self.ModuleRotationPhase` (select `bool` (>= _modulerotationphase 3) :`false` (+ _modulerotationphase 1)))
      (else
        (set `self.ModuleRotationPhase` (select `bool` (<= _modulerotationphase 0) :`false` (- _modulerotationphase 1) :`true` 3))))))

(fn `SpawnModule`
  (params (`Module Actor Class` :type "/Game/VesselEditor/ModuleBP Class Reference"))
  (`/Engine/EditorBlueprintResources/StandardMacros.IsValid` (`self.Current Module`)
    (:`Is Not Valid`
      (bind _returnvalue (`|SpawnActorFromClass` `Module Actor Class` (`KismetMathLibrary.MakeTransform` (`self.DeprojectMousePositionToWorld`)) "AlwaysSpawn" "OverrideRootScale" null null))
      (set `self.Current Module` _returnvalue))))

(fn `UserConstructionScript`)