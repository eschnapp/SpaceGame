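; ModuleBP is a vessel editor module actor that flags overlaps and snaps onto a vessel.
; On overlap it applies a dark red, translucent dynamic instance of the holo material and sets IsOverlapping; ending overlap clears both.
; HandleActorOverlap moves the module to the VesselBP root compartment's CS_1 socket when within 10 units, setting IsSnapping.
; The socket position is relative location plus actor location, ignoring rotation, and is checked only when overlap begins.
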(event `self.ReceiveBeginPlay`
  (`KismetSystemLibrary.PrintString` "Hello"))

(event `self.ReceiveActorBeginOverlap`
  (params (OtherActor :type "Actor Object Reference"))
  (`self.HandleActorOverlap` OtherActor)
  (bind _returnvalue (`KismetMaterialLibrary.CreateDynamicMaterialInstance` "/Game/VesselEditor/ModuleHoloMaterial.ModuleHoloMaterial" "None"))
  (`MaterialInstanceDynamic.SetVectorParameterValue` _returnvalue "Color" (struct :`R` 0.520833 :`B` 0.021455 :`A` 1.0))
  (`MaterialInstanceDynamic.SetScalarParameterValue` _returnvalue "Opacity" 0.75)
  (`PrimitiveComponent.SetMaterial` (`self.Module Static Mesh`) 0 _returnvalue)
  (set `self.IsOverlapping` true))

(event `self.ReceiveActorEndOverlap`
  (params (OtherActor :type "Actor Object Reference"))
  (`PrimitiveComponent.SetMaterial` (`self.Module Static Mesh`) 0 null)
  (set `self.IsOverlapping` false))

(fn `HandleActorOverlap`
  (params (OtherActor :type "Actor Object Reference"))
  (bind _asvessel_bp (cast `/Game/VesselEditor/VesselBP` OtherActor))
  (bind _returnvalue (+ (`StaticMeshSocket.RelativeLocation` (`StaticMesh.FindSocket` (`/Game/VesselEditor/VesselBP.RootCompartment` _asvessel_bp) "CS_1")) (`self.K2_GetActorLocation` _asvessel_bp)))
  (if (<= (`KismetMathLibrary.Vector_Distance` _returnvalue (`self.K2_GetActorLocation`)) 10.0)
    (set `self.IsSnapping` true)
    (`self.K2_SetActorLocation` _returnvalue)))

(fn `UserConstructionScript`)