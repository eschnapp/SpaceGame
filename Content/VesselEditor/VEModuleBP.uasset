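; Vessel editor module Blueprint that visually marks the module sitting at the grid's zero location.
; On custom initialization, it compares its grid coordinates on all three axes with the grid manager's zero location.
; On a match, it creates a dynamic material instance on the module's static mesh and sets its Color parameter to green.
; The construction script is empty.
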(event `self.CustomInitialization`
  (bind (__gridcoordinates_x __gridcoordinates_y __gridcoordinates_z) (break `IntVector` (`self._GridCoordinates`)))
  (bind __modulestaticmeshcomponent (`self._ModuleStaticMeshComponent`))
  (bind _returnvalue (`self.GetGridManager`))
  (bind (__gridzerolocation_x __gridzerolocation_y __gridzerolocation_z) (break `IntVector` (`VEGridManager._GridZeroLocation` _returnvalue)))
  (if (and (== __gridcoordinates_x __gridzerolocation_x) (== __gridcoordinates_y __gridzerolocation_y) (== __gridcoordinates_z __gridzerolocation_z))
    (bind _returnvalue_2 (`PrimitiveComponent.CreateDynamicMaterialInstance` __modulestaticmeshcomponent 0 (`PrimitiveComponent.GetMaterial` __modulestaticmeshcomponent 0) "None"))
    (`MaterialInstanceDynamic.SetVectorParameterValue` _returnvalue_2 "Color" (struct :`G` 0.552083 :`B` 0.099976 :`A` 1.0))))

(fn `UserConstructionScript`)