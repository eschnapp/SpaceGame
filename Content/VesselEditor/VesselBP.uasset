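; VesselBP is a modular vessel actor assembled from static mesh compartments joined at sockets.
; Its construction script creates the root compartment mesh, resets the Compartments list with it and records success in HasRootCompartment.
; AddCompartmentOld requires that root, snaps a new mesh to a parent socket, tracks it and reports success, while ignoring its own-socket parameter.
; AddModule attaches a supplied object to a mesh socket, keeping relative transforms.
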(fn `AddCompartment_Old`
  (params (`Compartment Mesh Class` :type "StaticMesh Object Reference") (`Compartment Mesh Socket Name` :type Name) (`Parent Mesh Instance` :type "StaticMeshComponent Object Reference") (`Parent Mesh Socket Name` :type Name))
  (returns (Success :type Boolean))
  (if (`self.HasRootCompartment`)
    (bind _returnvalue (`AddComponent|NODE_AddStaticMeshComponent-1` :`bManualAttachment` true :`RelativeTransform` (`KismetMathLibrary.MakeTransform` (0.0 0.0 0.0))))
    (bind _returnvalue_2 (`StaticMeshComponent.SetStaticMesh` _returnvalue `Compartment Mesh Class`))
    (if _returnvalue_2
      (bind _returnvalue_3 (`SceneComponent.K2_AttachToComponent` _returnvalue `Parent Mesh Instance` `Parent Mesh Socket Name` "SnapToTarget" "SnapToTarget" "SnapToTarget" true))
      (if _returnvalue_3
        (`KismetArrayLibrary.Array_Add` (`self.Compartments`) _returnvalue)
        (return true)
        (else
          (`ActorComponent.K2_DestroyComponent` _returnvalue)
          (`KismetSystemLibrary.PrintString` "Failed to attach to parent!")
          (return false)))
      (else
        (`KismetSystemLibrary.PrintString` "Failed to set the Static Mesh for this compartment!")
        (return false)))
    (else
      (`KismetSystemLibrary.PrintString` "No Root Compartment Found!")
      (return false))))

(fn `AddModule`
  (params (`AttachTo Mesh` :type "StaticMeshComponent Object Reference") (`AttachTo Socket Name` :type Name) (`Attached Actor` :type "Actor Object Reference"))
  (`self.K2_AttachToComponent` `Attached Actor` `AttachTo Mesh` `AttachTo Socket Name` "KeepRelative" "KeepRelative" "KeepRelative" true))

(fn `UserConstructionScript`
  (bind _compartments (`self.Compartments`))
  (bind _returnvalue (`AddComponent|NODE_AddStaticMeshComponent-0` :`RelativeTransform` (`KismetMathLibrary.MakeTransform` (0.0 0.0 0.0))))
  (`PrimitiveComponent.SetCollisionEnabled` _returnvalue "QueryAndPhysics")
  (bind _returnvalue_2 (`StaticMeshComponent.SetStaticMesh` _returnvalue (`self.RootCompartment`)))
  (if _returnvalue_2
    (`KismetArrayLibrary.Array_Clear` _compartments)
    (`KismetArrayLibrary.Array_Add` _compartments _returnvalue)
    (else
      (`KismetSystemLibrary.PrintString` "Failed to set RootCompartment mesh!")))
  (set `self.HasRootCompartment` _returnvalue_2))